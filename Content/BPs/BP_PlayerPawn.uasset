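; BP_PlayerPawn is the player pawn Blueprint, which passes its components up to parent-class setters.
; On BeginPlay it calls the parent, enables input for player controller 0, registers its skeletal mesh and pivot, then invokes the player pivot delegate.
; Getter functions expose the mesh and pivot.
; An aim montage call and construction-time pivot setup are left unconnected and never run.
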(event `self.ReceiveBeginPlay`
  (`parent.ReceiveBeginPlay`)
  (`|ExecutionSequence`
    (:`then_0`
      (`self.EnableInput` (`GameplayStatics.GetPlayerController` 0)))
    (:`then_1`
      (`self.SetSkeletalMeshComponent_CPP` (`self.SkeletalMesh`))
      (`self.SetPawnPivot` (`self.Pivot`))
      (`self.InvokePlayerPivotDelegate`))))

(event `InputAction|Use`
  (params (Key :type "Key Structure")))

(fn `GetPawnPivot`
  (returns (NewParam :type "SceneComponent Object Reference"))
  (return (`self.Pivot`)))

(fn `GetSkeletalMesh`
  (returns (SkeletalMeshComp :type "SkeletalMeshComponent Object Reference"))
  (return (`self.SkeletalMesh`)))

(fn `UserConstructionScript`)