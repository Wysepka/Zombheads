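; Player controller that possesses the PlayerPawn, views it through TPSCamera_BP and lets the player toggle a free spectator pawn.
; BeginPlay also sets the character pivot and caches the pawn's visual representation, which Tick rotates toward the mouse position.
; ChangeToSpectator spawns and possesses a SpectatorPawn_BP at the world origin; pressing again destroys it and reuses the BeginPlay possession and camera logic.
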(event `self.ReceiveTick`
  (params (DeltaSeconds :type "Float (single-precision)"))
  (`SceneComponent.K2_SetWorldRotation` (`self.PawnCharRepresentation`) (`self.RotationToMousePos`) false false))

(event `self.ReceiveBeginPlay`
  (`parent.ReceiveBeginPlay`)
  (`|ExecutionSequence`
    (:`then_0`
      (bind _returnvalue (`GameplayStatics.GetActorOfClass` "/Game/BPs/PlayerPawn.PlayerPawn_C" :!label _label))
      (`self.Possess` _returnvalue)
      (bind _returnvalue_2 (`GameplayStatics.GetActorOfClass` "/Game/BPs/TPSCamera_BP.TPSCamera_BP_C"))
      (`self.SetViewTargetWithBlend` _returnvalue_2))
    (:`then_1`
      (`self.SetCharacterObjPivot` (`self.CharacterPivot`)))
    (:`then_2`
      (bind _returnvalue_3 (`GameplayStatics.GetActorOfClass` "/Game/BPs/PlayerPawn.PlayerPawn_C"))
      (set `self.PawnCharRepresentation` (`/Game/BPs/PlayerPawn.PlayerRepresentation` _returnvalue_3)))))

(event `InputAction|ChangeToSpectator`
  (params (Key :type "Key Structure"))
  (:`Pressed`
    (if (`self.IsSpectating`)
      (`self.K2_DestroyActor` (`self.SpectateCamera`))
      (set `self.IsSpectating` false)
      (goto _label)
      (else
        (bind _returnvalue (`|SpawnActorFromClass` "/Game/BPs/SpectatorPawn_BP.SpectatorPawn_BP_C" (`KismetMathLibrary.MakeTransform` (0.0 0.0 0.0)) "Undefined" "OverrideRootScale" null null))
        (bind _output_get (set `self.SpectateCamera` _returnvalue))
        (set `self.IsSpectating` true)
        (`self.Possess` _output_get)
        (`KismetSystemLibrary.LogString` "Posessing SpectatorPawnBP")))))

(fn `UserConstructionScript`)