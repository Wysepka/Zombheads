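; Player controller that possesses the player pawn, views it through the third-person camera and toggles a spectator mode.
; BeginPlay finds the pawn and BP_TPSCamera by class, registers the default pawn and passes pivot references.
; ChangeToSpectator spawns and possesses a spectator pawn at world origin, or destroys it and reuses the BeginPlay possession path.
; Aim montage and pivot rotation nodes are disconnected.
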(event `self.ReceiveTick`
  (params (DeltaSeconds :type "Float (single-precision)")))

(event `self.ReceiveBeginPlay`
  (`parent.ReceiveBeginPlay`)
  (`|ExecutionSequence`
    (:`then_0`
      (bind _returnvalue (`GameplayStatics.GetActorOfClass` "/Game/BPs/BP_PlayerPawn.BP_PlayerPawn_C" :!label _label))
      (`|ExecutionSequence`
        (:`then_0`
          (`self.Possess` _returnvalue)
          (bind _returnvalue_2 (`GameplayStatics.GetActorOfClass` "/Game/BPs/BP_TPSCamera.BP_TPSCamera_C"))
          (`self.SetViewTargetWithBlend` _returnvalue_2))
        (:`then_1`
          (`self.SetDefaultPawn` _returnvalue)
          (set `self.DefaultPawnBP` _returnvalue))))
    (:`then_1`
      (`self.SetCharacterObjPivot` (`self.CharacterPivot`)))
    (:`then_2`
      (bind _returnvalue_3 (`GameplayStatics.GetActorOfClass` "/Game/BPs/BP_PlayerPawn.BP_PlayerPawn_C"))
      (bind _newparam (`/Game/BPs/BP_PlayerPawn.GetPawnPivot` _returnvalue_3))
      (set `self.PawnCharRepresentation` _newparam)
      (`KismetSystemLibrary.PrintString` "BeginPlay from BP"))))

(event `InputAction|ChangeToSpectator`
  (params (Key :type "Key Structure"))
  (:`Pressed`
    (if (`self.IsSpectating`)
      (`self.K2_DestroyActor` (`self.SpectateCamera`))
      (set `self.IsSpectating` false)
      (goto _label)
      (else
        (bind _returnvalue (`|SpawnActorFromClass` "/Game/BPs/BP_SpectatorPawn.BP_SpectatorPawn_C" (`KismetMathLibrary.MakeTransform` (0.0 0.0 0.0)) "Undefined" "MultiplyWithRoot" null null))
        (bind _output_get (set `self.SpectateCamera` _returnvalue))
        (set `self.IsSpectating` true)
        (`self.Possess` _output_get)
        (`KismetSystemLibrary.LogString` "Posessing SpectatorPawnBP")))))

(fn `UserConstructionScript`)